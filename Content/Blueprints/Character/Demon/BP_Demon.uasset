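; BP_Demon is a demon character that plays a summoning rise when spawned before becoming AI or default-controller driven.
; On BeginPlay it stores its spawn location and runs SummonTimeline, whose DistanceToRise track offsets the actor vertically without sweeping.
; When the timeline finishes, it sets mesh collision to query-only and spawns its default controller, deferring control until the rise ends.
; IsDead always returns false.
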(event EventBeginPlay
  (|CallParentFunction)
  (Variables|Default|SetSpawnLocation (Transformation|GetActorLocation))
  (bind _distancetorise (Timeline|SummonTimeline PlayFromStart)
    (:Update
      (Transformation|SetActorLocation self (+ (Variables|Default|GetSpawnLocation) (Math|Vector|MakeVector 0.0 0.0 _distancetorise)) false false))
    (:Finished
      (Collision|SetCollisionEnabled (Variables|Character|GetMesh) "QueryOnly")
      (Pawn|SpawnDefaultController))))

(fn ConstructionScript
  (|CallParentFunction))

(fn IsDead
  (return false))