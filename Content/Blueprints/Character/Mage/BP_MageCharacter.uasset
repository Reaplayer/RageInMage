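; BP_MageCharacter is the mage character Blueprint, handling attack facing, the attribute menu and camera zoom input.
; UpdateFacingTarget feeds a location to Motion Warping as the FacingTarget warp target.
; An input action toggles a newly created attribute menu widget, whose closed event resets the open flag.
; Two other input actions lengthen or shorten the spring arm by fixed, unclamped steps.
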(event Custom|AttributeMenuClosed_Event
  (Variables|Default|SetMenuActive false))

(event Input|EnhancedActionEvents|EnhancedInputActionIA_AttributeMenu
  (params (ActionValue :type Boolean) (ElapsedSeconds :type Float%20%28double-precision%29) (TriggeredSeconds :type Float%20%28double-precision%29) (InputAction :type Input%20Action%20Object%20Reference :default "/Game/Blueprints/Input/InputActions/IA_AttributeMenu.IA_AttributeMenu"))
  (if (Variables|Default|GetMenuActive)
    (Widget|RemovefromParent (Variables|Default|GetAttributeMenuWidget))
    (Variables|Default|SetMenuActive false)
    (else
      (bind _returnvalue (UserInterface|CreateWidget "/Game/Blueprints/UI/AttributeMenu/WBP_AttributeMenu.WBP_AttributeMenu_C" (Pawn|GetLocalViewingPlayerController self)))
      (bind _output_get (Variables|Default|SetAttributeMenuWidget _returnvalue))
      (UserInterface|Viewport|AddtoViewport _output_get 0)
      (Variables|Default|SetMenuActive true)
      (EventDispatchers|AssignAttributeMenuClosed _output_get (delegate Custom|AttributeMenuClosed_Event)))))

(event Input|EnhancedActionEvents|EnhancedInputActionIA_IncreaseCameraDistance
  (params (ActionValue :type Boolean) (ElapsedSeconds :type Float%20%28double-precision%29) (TriggeredSeconds :type Float%20%28double-precision%29) (InputAction :type Input%20Action%20Object%20Reference :default "/Game/Blueprints/Input/InputActions/IA_IncreaseCameraDistance.IA_IncreaseCameraDistance"))
  (bind _springarm (Variables|Default|GetSpringArm))
  (Variables|/Script/Engine.SpringArmComponent|SetTargetArmLength _springarm (+ (Variables|/Script/Engine.SpringArmComponent|GetTargetArmLength _springarm) 3e+02)))

(event Input|EnhancedActionEvents|EnhancedInputActionIA_DecreaseCameraDistance
  (params (ActionValue :type Boolean) (ElapsedSeconds :type Float%20%28double-precision%29) (TriggeredSeconds :type Float%20%28double-precision%29) (InputAction :type Input%20Action%20Object%20Reference :default "/Game/Blueprints/Input/InputActions/IA_DecreaseCameraDistance.IA_DecreaseCameraDistance"))
  (bind _springarm (Variables|Default|GetSpringArm))
  (Variables|/Script/Engine.SpringArmComponent|SetTargetArmLength _springarm (- (Variables|/Script/Engine.SpringArmComponent|GetTargetArmLength _springarm) 3e+02)))

(event EventUpdateFacingTarget
  (params (TargetLocation :type Vector%20%28by%20ref%29 :default "0, 0, 0"))
  (Class|MotionWarpingComponent|AddorUpdateWarpTargetfromLocation (Variables|Default|GetMotionWarping) "FacingTarget" TargetLocation))

(fn ConstructionScript)