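; BP_Goblin_Shaman is a goblin shaman character that tracks how many summoned minions it has.
; Registering a spawned minion casts it to BP_Summon, binds to its decrement-summon-count event and increments the count.
; A minion death event decrements the count, and both paths write the new value to a Blackboard key for the AI to read.
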(event Custom|OnMinionDeath
  (bind _returnvalue (Class|CombatInterface|GetSummonCount))
  (bind _result (Math|Integer|DecrementInt _returnvalue)
    (:%20%20
      (Class|CombatInterface|SetSummonCount _result)
      (Class|BlackboardComponent|SetValueasInt (AI|GetBlackboard 0) (Variables|Default|GetBlackboardSummonCountKey) _result))))

(event EventRegisterSpawnedMinion
  (params (Minion :type Actor%20Object%20Reference))
  (bind _asbp_summon (Utilities|Casting|CastToBP_Summon Minion))
  (CallFunction|RegisterMinion _asbp_summon))

(fn ConstructionScript
  (|CallParentFunction))

(fn RegisterMinion
  (params (NewSummon :type BP%20Summon%20Object%20Reference))
  (EventDispatchers|BindEventtoDecrementSummonCount NewSummon (EventDispatchers|CreateEvent :!event Custom|OnMinionDeath))
  (bind _returnvalue (Class|CombatInterface|GetSummonCount))
  (bind _result (Math|Integer|IncrementInt _returnvalue)
    (:%20%20
      (Class|CombatInterface|SetSummonCount _result)
      (Class|BlackboardComponent|SetValueasInt (AI|GetBlackboard 0) (Variables|Default|GetBlackboardSummonCountKey) _result))))