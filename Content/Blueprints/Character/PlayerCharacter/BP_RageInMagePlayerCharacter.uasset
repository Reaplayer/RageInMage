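; Player character Blueprint for RageInMage, handling the tabbed menu, camera zoom and motion-warp facing.
; The attribute menu input creates or removes a tabbed menu widget, switching input mode and offsetting its screen position by local player index.
; Camera distance inputs step the spring arm length in or out while the menu is closed.
; UpdateFacingTarget feeds a location to Motion Warping as the FacingTarget warp target.
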(event Input|EnhancedActionEvents|EnhancedInputActionIA_AttributeMenu
  (params (ActionValue :type Boolean) (ElapsedSeconds :type Float%20%28double-precision%29) (TriggeredSeconds :type Float%20%28double-precision%29) (InputAction :type Input%20Action%20Object%20Reference :default "/Game/Blueprints/Input/InputActions/IA_AttributeMenu.IA_AttributeMenu"))
  (if (Variables|Default|GetMenuActive)
    (Widget|RemovefromParent (Variables|Default|GetTabbedMenu))
    (Variables|Default|SetMenuActive false)
    (Input|SetInputModeGameOnly (Pawn|GetLocalViewingPlayerController) false)
    (else
      (bind _returnvalue (UserInterface|CreateWidget "/Game/Blueprints/UI/TabbedMenu/WBP_TabbedMenu.WBP_TabbedMenu_C" (Pawn|GetLocalViewingPlayerController)))
      (bind _output_get (Variables|Default|SetTabbedMenu _returnvalue))
      (Variables|/Game/Blueprints/UI/TabbedMenu/WBP_TabbedMenu.WBP_TabbedMenu_C|SetBP_RageInMagePlayerCharacter _output_get self)
      (UserInterface|Viewport|AddtoViewport _output_get 0)
      (Variables|Default|SetMenuActive true)
      (Class|UserWidget|SetPositioninViewport (Variables|Default|GetTabbedMenu) (Math|Vector2D|MakeVector2D (Math|Conversions|ToFloat(Integer) (* 480 (Class|RageinMageAbilitySystemLibrary|GetLocalPlayerIndex (Pawn|GetLocalViewingPlayerController)))) (- (.Y (Math|Vector2D|BreakVector2D (Viewport|GetViewportSize))) 385.0)) true)
      (Input|SetInputModeGameandUI (Pawn|GetLocalViewingPlayerController) (Variables|Default|GetTabbedMenu) "DoNotLock" true false))))

(event Input|EnhancedActionEvents|EnhancedInputActionIA_IncreaseCameraDistance
  (params (ActionValue :type Boolean) (ElapsedSeconds :type Float%20%28double-precision%29) (TriggeredSeconds :type Float%20%28double-precision%29) (InputAction :type Input%20Action%20Object%20Reference :default "/Game/Blueprints/Input/InputActions/IA_IncreaseCameraDistance.IA_IncreaseCameraDistance"))
  (if (not (Variables|Default|GetMenuActive))
    (Variables|/Script/Engine.SpringArmComponent|SetTargetArmLength (Variables|Default|GetCameraBoom) (+ (Variables|/Script/Engine.SpringArmComponent|GetTargetArmLength (Variables|Default|GetCameraBoom)) 3e+02))))

(event Input|EnhancedActionEvents|EnhancedInputActionIA_DecreaseCameraDistance
  (params (ActionValue :type Boolean) (ElapsedSeconds :type Float%20%28double-precision%29) (TriggeredSeconds :type Float%20%28double-precision%29) (InputAction :type Input%20Action%20Object%20Reference :default "/Game/Blueprints/Input/InputActions/IA_DecreaseCameraDistance.IA_DecreaseCameraDistance"))
  (if (not (Variables|Default|GetMenuActive))
    (Variables|/Script/Engine.SpringArmComponent|SetTargetArmLength (Variables|Default|GetCameraBoom) (- (Variables|/Script/Engine.SpringArmComponent|GetTargetArmLength (Variables|Default|GetCameraBoom)) 3e+02))))

(event EventUpdateFacingTarget
  (params (TargetLocation :type Vector%20%28by%20ref%29 :default "0, 0, 0"))
  (Class|MotionWarpingComponent|AddorUpdateWarpTargetfromLocation (Variables|Default|GetMotionWarping) "FacingTarget" TargetLocation))

(fn ConstructionScript)