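; Server-side enemy spawner that runs escalating waves, starting on BeginPlay when AutoStart is set.
; Each wave grows linearly and spawns random EnemyClasses at random reachable navmesh points around the spawner, skipping spawns once MaxAliveEnemies is reached.
; A looping timer polls the world-wide RageInMageEnemyCharacter count and schedules the next wave after a delay when none remain.
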(event Custom|StartNextWave
  (Variables|Default|SetCurrentWave (+ (Variables|Default|GetCurrentWave) 1))
  (for _index (range 1 (+ (* (- (Variables|Default|GetCurrentWave) 1) (Variables|Default|GetWaveSizeIncrement)) (Variables|Default|GetEnemiesPerWave)))
    (CallFunction|SpawnOneEnemy))
  (Variables|Default|SetbWaveActive true))

(event Custom|CheckWaveCleared
  (if (Variables|Default|GetbWaveActive)
    (bind _outactors (Actor|GetAllActorsOfClass "/Script/RageInMage.RageInMageEnemyCharacter"))
    (if (<= (Utilities|Array|Length _outactors) 0)
      (Variables|Default|SetbWaveActive false)
      (Utilities|Time|SetTimerbyFunctionName 0 "StartNextWave" (Variables|Default|GetTimeBetweenWaves)))))

(event EventBeginPlay
  (if (Ability|HasAuthority)
    (if (Variables|Default|GetbAutoStart)
      (Utilities|Time|SetTimerbyFunctionName 0 "CheckWaveCleared" 1.0 true)
      (CallFunction|StartNextWave))))

(event Collision|EventActorBeginOverlap
  (params (OtherActor :type Actor%20Object%20Reference)))

(event EventTick
  (params (DeltaSeconds :type Float%20%28single-precision%29)))

(fn ConstructionScript)

(fn SpawnOneEnemy
  (bind _returnvalue (Transformation|GetActorLocation))
  (bind _spawnradius (Variables|Default|GetSpawnRadius))
  (bind _enemyclasses (Variables|Default|GetEnemyClasses))
  (bind (_randomlocation _returnvalue_2) (AI|Navigation|GetRandomReachablePointinRadius _returnvalue _spawnradius 0 0))
  (bind _outactors (Actor|GetAllActorsOfClass "/Script/RageInMage.RageInMageEnemyCharacter"))
  (if (< (Utilities|Array|Length _outactors) (Variables|Default|GetMaxAliveEnemies))
    (if _returnvalue_2
      (Game|SpawnActorfromClass (Utilities|Array|Get(acopy) _enemyclasses (Math|Random|RandomInteger (Utilities|Array|Length _enemyclasses))) (Math|Transform|MakeTransform _randomlocation) "AdjustIfPossibleButAlwaysSpawn" "MultiplyWithRoot" 0 0))))