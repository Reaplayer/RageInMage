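; GA_SimpleIce is the player's water-class Simple Ice ability, an aimed attack that fires a spread of BP_SimpleIce projectiles.
; While aiming, an AimMode task drives spread indicators tinted in the class colour.
; On release it commits cost, turns the avatar to the target, spawns projectiles from the weapon socket, then commits cooldown.
; Cancelling clears indicators and ends the ability; the montage-and-event path is disconnected.
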(event Ability|EventActivateAbility
  (bind _aimposition (|AimModeTask (Variables|Default|GetAimIndicatorLength))
    (:OnAimUpdate
      (if (Class|RageinMageSpreadProjectileSpell|HasActiveSpreadIndicators)
        _
        (else
          (bind _returnvalue (Class|CombatInterface|GetCharacterClass(Message) (Ability|GetAvatarActorfromActorInfo)))
          (Class|RageinMageSpreadProjectileSpell|SpawnSpreadIndicators "/Game/RageInMageSpells/VFX/Aim/NS_Aim_Line_Water.NS_Aim_Line_Water" (Class|RageinMageAbilitySystemLibrary|GetClassProgressBarColor _returnvalue))))
      (Class|RageinMageSpreadProjectileSpell|UpdateSpreadIndicators _aimposition))
    (:OnInputReleased
      (Class|RageinMageSpreadProjectileSpell|DestroySpreadIndicators)
      (bind _returnvalue_2 (Ability|CommitAbilityCost false))
      (if _returnvalue_2
        (Class|CombatInterface|UpdateFacingTarget(Message) (Ability|GetAvatarActorfromActorInfo) _aimposition)
        (Class|RageinMageSpreadProjectileSpell|SpawnSpreadProjectiles _aimposition (GameplayTags|MakeLiteralGameplayTag "(TagName=\"CombatSocket.Weapon\")") "/Game/Blueprints/AbilitySystem/Player/Abilities/Water/SimpleIce/BP_SimpleIce.BP_SimpleIce_C" false)
        (Ability|CommitAbilityCooldown false)
        (Ability|EndAbility)
        (else
          (Ability|EndAbility))))
    (:OnCancelled
      (Class|RageinMageSpreadProjectileSpell|DestroySpreadIndicators)
      (Ability|EndAbility))))