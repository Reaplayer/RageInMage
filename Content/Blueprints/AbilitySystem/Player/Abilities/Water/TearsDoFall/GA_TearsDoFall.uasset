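; GA_TearsDoFall is a player Water gameplay ability that places an ice storm zone at an aimed position.
; An AimModeTask runs the aiming, and releasing the input commits the cost, turns the avatar toward the target and spawns BP_IceStormZone there.
; Cooldown is committed only after the spawn, so cancelling or failing the cost check ends the ability without starting it.
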(event Ability|EventOnEndAbility
  (params (bWasCancelled :type Boolean)))

(event Ability|EventActivateAbility
  (bind _aimposition (|AimModeTask (Variables|Default|GetAimIndicatorLength))
    (:OnInputReleased
      (bind _returnvalue (Ability|CommitAbilityCost false))
      (if _returnvalue
        (Class|CombatInterface|UpdateFacingTarget(Message) (Ability|GetAvatarActorfromActorInfo) _aimposition)
        (Game|SpawnActorfromClass "/Game/Blueprints/AbilitySystem/Player/Abilities/Water/TearsDoFall/BP_IceStormZone.BP_IceStormZone_C" (Math|Transform|MakeTransform _aimposition) "Undefined" "MultiplyWithRoot" 0)
        (Ability|CommitAbilityCooldown false)
        (Ability|EndAbility)
        (else
          (Ability|EndAbility))))
    (:OnCancelled
      (Ability|EndAbility))))