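; Gameplay ability for the player's Riding Tide water skill, which starts a surf toward an aimed position.
; An aim-mode task shows the indicator until input release, then the ability commits cost, updates the avatar's facing and passes the offset to the aim point to BeginSurf.
; Cooldown is force-committed only after surfing begins.
; Cancelled aim or failed cost ends the ability.
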(event Ability|EventOnEndAbility
  (params (bWasCancelled :type Boolean))
  (Ability|EndAbility))

(event Ability|EventActivateAbility
  (bind _aimposition (|AimModeTask (Variables|Default|GetAimIndicatorLength))
    (:OnInputReleased
      (bind _returnvalue (Ability|CommitAbilityCost false))
      (if _returnvalue
        (Class|CombatInterface|UpdateFacingTarget(Message) (Ability|GetAvatarActorfromActorInfo) _aimposition)
        (Class|RageinMageSurfAbility|BeginSurf (- _aimposition (Transformation|GetActorLocation (Ability|GetAvatarActorfromActorInfo))))
        (Ability|CommitAbilityCooldown false true)
        (else
          (Ability|EndAbility))))
    (:OnCancelled
      (Ability|EndAbility))))