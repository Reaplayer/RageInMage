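; Player water gameplay ability that raises a Soothing Bubble shield on the avatar.
; Activation commits cost, then calls ActivateShield and commits cooldown, or ends the ability if the cost commit fails.
; Shield logic lives outside this graph, which handles its events for visuals only.
; The activated event attaches the AquaShield Niagara effect to the character mesh, and the absorbed or expired events destroy it.
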(event EventOnShieldActivated
  (bind _ascharacter (Utilities|Casting|CastToCharacter (Ability|GetAvatarActorfromActorInfo)))
  (bind _returnvalue (Niagara|SpawnSystemAttached "/Game/MegaMagicVFXBundle/VFX/MagicShieldsVFX/VFX/DefaultVersions/AquaShield/Systems/N_AquaShield.N_AquaShield" (Variables|/Script/Engine.Character|GetMesh _ascharacter) "None" "0, 0, 0" "0, 0, 0" "KeepRelativeOffset" false))
  (Variables|VFX|SetShieldVFXComponent _returnvalue))

(event EventOnShieldAbsorbed
  (params (AbsorbedDamage :type Float%20%28single-precision%29))
  (bind _shieldvfxcomponent (Variables|VFX|GetShieldVFXComponent))
  (Utilities|IsValid _shieldvfxcomponent
    (:Is%20Valid
      (Components|DestroyComponent _shieldvfxcomponent))))

(event Ability|EventActivateAbility
  (bind _returnvalue (Ability|CommitAbilityCost false))
  (if _returnvalue
    (Class|RageinMageShieldAbility|ActivateShield)
    (Ability|CommitAbilityCooldown false)
    (else
      (Ability|EndAbility))))

(event EventOnShieldExpired
  (bind _shieldvfxcomponent (Variables|VFX|GetShieldVFXComponent))
  (Utilities|IsValid _shieldvfxcomponent
    (:Is%20Valid
      (Components|DestroyComponent _shieldvfxcomponent))))