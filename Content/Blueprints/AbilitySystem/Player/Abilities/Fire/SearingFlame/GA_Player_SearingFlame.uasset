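; Player gameplay ability for Searing Flame, an aimed fire projectile cast.
; While aiming, an aim task drives a lazily spawned line decal, projected downward and oriented from the avatar toward the aim point.
; On release, it removes the decal, commits, turns the avatar toward the target and plays the cast montage.
; A montage gameplay event spawns BP_SearingFlame from the weapon socket toward the aim point, and montage end or aim cancel ends the ability.
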(event Ability|EventActivateAbility
  (bind _returnvalue (Ability|GetAvatarActorfromActorInfo))
  (bind _indicatorforwardoffset (Variables|Default|GetIndicatorForwardOffset))
  (bind _returnvalue_2 (Transformation|GetActorLocation _returnvalue))
  (bind _aimposition (|AimModeTask (Variables|Default|GetAimIndicatorLength))
    (:OnAimUpdate
      (Utilities|IsValid (Variables|Indicator|GetIndicatorDecal)
        (:Is%20Valid
          _)
        (:Is%20Not%20Valid
          (bind _returnvalue_3 (Rendering|Decal|SpawnDecalatLocation "/Game/Blueprints/AbilitySystem/Player/Abilities/M_AimLine_Decal.M_AimLine_Decal" (Math|Vector|MakeVector 128.0 (Variables|Default|GetAimIndicatorWidth) (Variables|Default|GetAimIndicatorLength)) (Transformation|GetActorLocation (Ability|GetAvatarActorfromActorInfo)) "-90.000000,0.000000,0.000000" 0.0))
          (bind _output_get (Variables|Indicator|SetIndicatorDecal _returnvalue_3))
          (bind _returnvalue_4 (Rendering|Material|CreateDynamicMaterialInstance _output_get :!class /Script/Engine.DecalComponent))
          (Variables|Indicator|SetDecalDynamicMaterial _returnvalue_4)))
      (Transformation|SetWorldLocationAndRotation (Variables|Indicator|GetIndicatorDecal) (+ (* (Transformation|GetActorForwardVector (Ability|GetAvatarActorfromActorInfo)) (Math|Vector|MakeVector _indicatorforwardoffset _indicatorforwardoffset 0.0)) (+ (* (Class|KismetMathLibrary|VectorNormal2D (- _aimposition _returnvalue_2) 0.0001) (Variables|Default|GetAimIndicatorLength)) _returnvalue_2)) (Math|Rotator|MakeRotator 0.0 -9e+01 (.Yaw (Math|Rotator|BreakRotator (Math|Rotator|FindLookatRotation _returnvalue_2 _aimposition)))) false false))
    (:OnInputReleased
      (Utilities|IsValid (Variables|Indicator|GetIndicatorDecal)
        (:Is%20Valid
          (Components|DestroyComponent (Variables|Indicator|GetIndicatorDecal)))
        (:Is%20Not%20Valid
          _))
      (bind _returnvalue_5 (Ability|CommitAbility))
      (if _returnvalue_5
        (Class|CombatInterface|UpdateFacingTarget(Message) (Ability|GetAvatarActorfromActorInfo) _aimposition)
        (|PlayMontageandWaitProxy "None" "/Game/Assets/Characters/Aura/Animations/Abilities/AM_Cast_SearingFlame.AM_Cast_SearingFlame" 1.0 "None" false 1.0 0.0 false
          (:then
            (Ability|Tasks|WaitGameplayEvent "(TagName=\"Event.Montage.SearingFlame\")" 0 true
              (:EventReceived
                (Class|RageinMageProjectileSpell|SpawnProjectile _aimposition (GameplayTags|MakeLiteralGameplayTag "(TagName=\"CombatSocket.Weapon\")") "/Game/Blueprints/AbilitySystem/Player/Abilities/Fire/SearingFlame/BP_SearingFlame.BP_SearingFlame_C" false 0))))
          (:OnCompleted
            (Ability|EndAbility :!label _label))
          (:OnBlendOut
            (goto _label))
          (:OnInterrupted
            (goto _label))
          (:OnCancelled
            (goto _label)))))
    (:OnCancelled
      (Utilities|IsValid (Variables|Indicator|GetIndicatorDecal)
        (:Is%20Valid
          (Components|DestroyComponent (Variables|Indicator|GetIndicatorDecal)))
        (:Is%20Not%20Valid
          _))
      (Ability|EndAbility))))