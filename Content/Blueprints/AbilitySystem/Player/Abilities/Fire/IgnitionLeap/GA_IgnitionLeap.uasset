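; Fire player ability Ignition Leap that launches the character to an aimed point and triggers an explosion on landing.
; While aiming, an aim task drives a ground decal scaled to the explosion radius and a leap arc drawn with debug lines.
; On release it commits, faces the target and launches with a calculated velocity.
; A return to Walking movement mode triggers the explosion and ends the ability; cancelling or failed commit just ends it.
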(event Ability|EventActivateAbility
  (bind _aimindicatorradius (Variables|Default|GetAimIndicatorRadius))
  (bind _aimposition (|AimModeTask (Variables|Default|GetMaxSpellRange))
    (:OnAimUpdate
      (Utilities|IsValid (Variables|Default|GetIndicatorDecal)
        (:Is%20Valid
          _)
        (:Is%20Not%20Valid
          (bind _returnvalue (Rendering|Decal|SpawnDecalatLocation "/Game/Blueprints/AbilitySystem/Player/Abilities/M_AimCircle_Decal.M_AimCircle_Decal" (Math|Vector|MakeVector _aimindicatorradius _aimindicatorradius 2e+02) (Transformation|GetActorLocation (Ability|GetAvatarActorfromActorInfo)) "0.000000,0.000000,-90.000000" 0.0))
          (bind _output_get (Variables|Default|SetIndicatorDecal _returnvalue))
          (bind _returnvalue_2 (Rendering|Material|CreateDynamicMaterialInstance _output_get :!class /Script/Engine.DecalComponent))
          (bind _output_get_2 (Variables|Default|SetDecalDynamicMaterial _returnvalue_2))
          (Rendering|Material|SetScalarParameterValue _output_get_2 "Radius" (.Value (Utilities|Struct|BreakScalableFloat (Variables|Default|GetExplosionRadius))) :!class /Script/Engine.MaterialInstanceDynamic)))
      (Transformation|SetWorldLocationAndRotation (Variables|Default|GetIndicatorDecal) _aimposition "0, 0, 0" false false)
      (for (_ _array_index) (Class|RageinMageLeapAbility|GetLeapArcPreviewPoints _aimposition 30)
        (if (< _array_index (Utilities|Array|LastIndex (Class|RageinMageLeapAbility|GetLeapArcPreviewPoints _aimposition 30)))
          (Rendering|Debug|DrawDebugLine (Utilities|Array|Get(acopy) (Class|RageinMageLeapAbility|GetLeapArcPreviewPoints _aimposition 30) _array_index) (Utilities|Array|Get(acopy) (Class|RageinMageLeapAbility|GetLeapArcPreviewPoints _aimposition 30) (+ _array_index 1)) "(R=1.0,G=0.5,B=0.0,A=1.0)" 0.0 2.0))))
    (:OnInputReleased
      (Utilities|IsValid (Variables|Default|GetIndicatorDecal)
        (:Is%20Valid
          (Components|DestroyComponent (Variables|Default|GetIndicatorDecal)))
        (:Is%20Not%20Valid
          _))
      (bind _returnvalue_3 (Ability|CommitAbility))
      (if _returnvalue_3
        (Class|CombatInterface|UpdateFacingTarget(Message) (Ability|GetAvatarActorfromActorInfo) _aimposition)
        (bind _ascharacter (Utilities|Casting|CastToCharacter (Ability|GetAvatarActorfromActorInfo)))
        (Character|LaunchCharacter _ascharacter (Class|RageinMageLeapAbility|CalculateLaunchVelocitytoTarget _aimposition) true true)
        (Ability|Tasks|WaitMovementModeChange "MOVE_Walking"
          (:OnChange
            (Class|RageinMageLeapAbility|ApplyLandingExplosion)
            (Ability|EndAbility)))
        (else
          (Ability|EndAbility))))
    (:OnCancelled
      (Utilities|IsValid (Variables|Default|GetIndicatorDecal)
        (:Is%20Valid
          (Components|DestroyComponent (Variables|Default|GetIndicatorDecal)))
        (:Is%20Not%20Valid
          _))
      (Ability|EndAbility))))