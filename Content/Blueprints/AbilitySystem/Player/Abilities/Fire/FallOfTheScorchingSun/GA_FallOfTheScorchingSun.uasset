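; Player fire Gameplay Ability that lets the player aim an area within max spell range and call down a meteor rain there.
; An AimModeTask drives a lazily spawned indicator decal, sized to the aim radius, that follows the aim position.
; Releasing input removes the decal, commits the ability, turns the avatar toward the target and calls BeginMeteorRain.
; Cancelling or a failed commit ends the ability without casting.
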(event Ability|EventActivateAbility
  (bind _aimindicatorradius (Variables|Default|GetAimIndicatorRadius))
  (bind _aimposition (|AimModeTask (Variables|Default|GetMaxSpellRange))
    (:OnAimUpdate
      (Utilities|IsValid (Variables|Default|GetIndicatorDecal)
        (:Is%20Valid
          _)
        (:Is%20Not%20Valid
          (bind _returnvalue (Rendering|Decal|SpawnDecalatLocation "/Game/Mixed_Magic_VFX_Pack/Materials/Instance_Materials/MI_Decal_Inst_1.MI_Decal_Inst_1" (Math|Vector|MakeVector _aimindicatorradius _aimindicatorradius 0.0) (Transformation|GetActorLocation (Ability|GetAvatarActorfromActorInfo)) "-90.000000,0.000000,0.000000" 0.0))
          (bind _output_get (Variables|Default|SetIndicatorDecal _returnvalue))
          (bind _returnvalue_2 (Rendering|Material|CreateDynamicMaterialInstance _output_get :!class /Script/Engine.DecalComponent))
          (Variables|Default|SetDecalDynamicMaterial _returnvalue_2)))
      (Transformation|SetWorldLocationAndRotation (Variables|Default|GetIndicatorDecal) _aimposition "0, 0, 0" false false))
    (:OnInputReleased
      (Utilities|IsValid (Variables|Default|GetIndicatorDecal)
        (:Is%20Valid
          (Components|DestroyComponent (Variables|Default|GetIndicatorDecal)))
        (:Is%20Not%20Valid
          _))
      (bind _returnvalue_3 (Ability|CommitAbility))
      (if _returnvalue_3
        (Class|CombatInterface|UpdateFacingTarget(Message) (Ability|GetAvatarActorfromActorInfo) _aimposition)
        (Class|RageinMageMeteorAbility|BeginMeteorRain _aimposition)
        (Ability|EndAbility)
        (else
          (Ability|EndAbility))))
    (:OnCancelled
      (Utilities|IsValid (Variables|Default|GetIndicatorDecal)
        (:Is%20Valid
          (Components|DestroyComponent (Variables|Default|GetIndicatorDecal)))
        (:Is%20Not%20Valid
          _))
      (Ability|EndAbility))))