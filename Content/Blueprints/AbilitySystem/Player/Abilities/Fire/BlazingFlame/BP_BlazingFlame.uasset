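; BP_BlazingFlame is an actor for the player's Blazing Flame fire ability that detects overlaps and currently only visualizes them.
; On BeginPlay it sets its Sphere collision to query-only.
; Overlaps with actors other than its owner run a zero-length Visibility line trace at the actor's location and draw a debug sphere at the returned impact point.
; It applies no damage or effects.
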(event EventBeginPlay
  (Collision|SetCollisionEnabled (Variables|Default|GetSphere) "QueryOnly"))

(event Collision|EventActorBeginOverlap
  (params (OtherActor :type Actor%20Object%20Reference))
  (if (not (== OtherActor (Components|GetOwner)))
    (bind _outhit (Collision|LineTraceByChannel (Transformation|GetActorLocation) (Transformation|GetActorLocation) "TraceTypeQuery1" false 0 "ForDuration"))
    (Rendering|Debug|DrawDebugSphere (.ImpactPoint (Collision|BreakHitResult _outhit)) 1e+02 100 "(R=1.000000,G=0.000000,B=0.000000,A=1.000000)" 5.0)))

(fn ConstructionScript)