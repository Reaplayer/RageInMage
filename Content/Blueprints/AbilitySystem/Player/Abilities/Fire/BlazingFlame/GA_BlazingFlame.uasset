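; Player Gameplay Ability for Blazing Flame, a charged fire spell aimed at a landing point within max range.
; After committing cost, an AimModeTask updates charge and indicator; input release fires at the last landing location, cancel aborts, and both commit cooldown.
; Charge callbacks drive a Niagara aim circle tinted by character class and sized to the explosion radius.
; The aim arc is drawn with debug lines.
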(event Ability|EventActivateAbility
  (bind _returnvalue (GameplayTags|MakeLiteralGameplayTag "(TagName=\"CombatSocket.Weapon\")"))
  (bind _returnvalue_2 (Ability|CommitAbilityCost false))
  (if _returnvalue_2
    (Class|RageinMageChargedSpell|BeginCharge _returnvalue)
    (bind (_asynctaskproxy _aimposition _deltatime) (|AimModeTask (Variables|Default|GetMaxSpellRange))
      (:OnAimUpdate
        (bind _returnvalue_3 (Class|RageinMageChargedSpell|UpdateChargeandIndicator _deltatime _aimposition _returnvalue))
        (Variables|Indicator|SetLastLandingLocation _returnvalue_3))
      (:OnInputReleased
        (Class|RageinMageChargedSpell|ReleaseChargedSpell (Variables|Indicator|GetLastLandingLocation) _returnvalue)
        (Ability|CommitAbilityCooldown false true)
        (Ability|EndAbility))
      (:OnCancelled
        (Class|RageinMageChargedSpell|CancelCharge)
        (Ability|CommitAbilityCooldown false true)
        (Ability|EndAbility)))
    (else
      (Ability|EndAbility))))

(event Ability|EventOnEndAbility
  (params (bWasCancelled :type Boolean)))

(event EventOnChargeBegin
  (bind _returnvalue (Ability|GetAvatarActorfromActorInfo))
  (bind _returnvalue_2 (Niagara|SpawnSystematLocation "/Game/RageInMageSpells/VFX/Aim/NS_Aim_Circle.NS_Aim_Circle" (Variables|Indicator|GetLastLandingLocation) "0, 0, 0" "1.000000,1.000000,1.000000" false))
  (bind _output_get (Variables|Indicator|SetIndicatorVFX _returnvalue_2))
  (Niagara|SetNiagaraVariable(Float) _output_get "Radius" (.Value (Utilities|Struct|BreakScalableFloat (Variables|Default|GetImpactExplosionRadius))))
  (bind _returnvalue_3 (Class|CombatInterface|GetCharacterClass(Message) _returnvalue))
  (bind _returnvalue_4 (Class|RageinMageAbilitySystemLibrary|GetCharacterClassInfo _returnvalue))
  (Niagara|SetNiagaraVariable(LinearColor) (Variables|Indicator|GetIndicatorVFX) "RingColour" (.SpecifiedColor (Utilities|Struct|BreakSlateColor (Utilities|Struct|BreakCharacterClassDefaultInfo (Class|CharacterClassInfo|GetCharacterClassDefaultInfo _returnvalue_4 _returnvalue_3))))))

(event EventOnChargeUpdate
  (params (LandingLocation :type Vector%20%28by%20ref%29 :default "0, 0, 0") (ChargePercent :type Float%20%28single-precision%29) (IndicatorRadius :type Float%20%28single-precision%29) (ArcPoints :type Array%20of%20Vectors))
  (bind _indicatorvfx (Variables|Indicator|GetIndicatorVFX))
  (Utilities|IsValid _indicatorvfx
    (:Is%20Valid
      (Transformation|SetWorldLocation _indicatorvfx LandingLocation false false)
      (Niagara|SetNiagaraVariable(Float) _indicatorvfx "Radius" IndicatorRadius)
      (for (_ _array_index) ArcPoints
        (if (< _array_index (Utilities|Array|LastIndex ArcPoints))
          (Rendering|Debug|DrawDebugLine (Utilities|Array|Get(acopy) ArcPoints _array_index) (Utilities|Array|Get(acopy) ArcPoints (+ _array_index 1)) "(R=1.0,G=0.4,B=0.0,A=1.0)" 0.0 3.0))))))

(event EventOnChargeEnd
  (Utilities|IsValid (Variables|Indicator|GetIndicatorVFX)
    (:Is%20Valid
      (Components|Activation|Deactivate (Variables|Indicator|GetIndicatorVFX))
      (Components|DestroyComponent (Variables|Indicator|GetIndicatorVFX))
      (Variables|Indicator|SetIndicatorVFX 0))))