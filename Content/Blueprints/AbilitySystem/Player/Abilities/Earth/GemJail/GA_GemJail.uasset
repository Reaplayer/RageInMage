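; Player Earth gameplay ability, Gem Jail, that places a petrifying zone at an aimed position.
; An AimMode task runs on activation; releasing input commits the ability cost only, without committing cooldown here.
; On success it spawns BP_GemJailZone at the aim position, owned and instigated by the avatar pawn, passing in petrify delay and duration.
; The ability then ends, as it does on failed commit or cancelled aim.
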(event Ability|EventActivateAbility
  (bind _returnvalue (Ability|GetAvatarActorfromActorInfo))
  (bind _aimposition (|AimModeTask (Variables|Default|GetAimIndicatorLength))
    (:OnInputReleased
      (bind _returnvalue_2 (Ability|CommitAbilityCost false))
      (if _returnvalue_2
        (bind _aspawn (Utilities|Casting|CastToPawn _returnvalue))
        (Game|SpawnActorfromClass :Class "/Game/Blueprints/AbilitySystem/Player/Abilities/Earth/GemJail/BP_GemJailZone.BP_GemJailZone_C" :SpawnTransform (Math|Transform|MakeTransform _aimposition) :CollisionHandlingOverride "Undefined" :TransformScaleMethod "MultiplyWithRoot" :Owner _returnvalue :PetrifyDelay 2.0 :PetrifyDuration 4.0 :Instigator _aspawn)
        (Ability|EndAbility)
        (else
          (Ability|EndAbility))))
    (:OnCancelled
      (Ability|EndAbility))))

(event Ability|EventOnEndAbility
  (params (bWasCancelled :type Boolean))
  (Ability|EndAbility))