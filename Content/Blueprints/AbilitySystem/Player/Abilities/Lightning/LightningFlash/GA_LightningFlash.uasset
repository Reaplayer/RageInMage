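; GA_LightningFlash is a player lightning gameplay ability that is aimed before it fires.
; On activation an AimModeTask shows aiming with a set indicator length until input is released or cancelled.
; On release, if the cost commits, it turns the avatar toward the aim position, calls ApplyLightningFlash there and commits the cooldown.
; Every path ends the ability, and cost and cooldown commit separately, so cancelling spends neither.
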(event Ability|EventActivateAbility
  (bind _aimposition (|AimModeTask (Variables|Default|GetAimIndicatorLength))
    (:OnInputReleased
      (bind _returnvalue (Ability|CommitAbilityCost false))
      (if _returnvalue
        (Class|CombatInterface|UpdateFacingTarget(Message) (Ability|GetAvatarActorfromActorInfo) _aimposition)
        (Class|RageinMageLightningFlashAbility|ApplyLightningFlash _aimposition)
        (Ability|CommitAbilityCooldown false)
        (Ability|EndAbility)
        (else
          (Ability|EndAbility))))
    (:OnCancelled
      (Ability|EndAbility))))

(event Ability|EventOnEndAbility
  (params (bWasCancelled :type Boolean))
  (Ability|EndAbility))