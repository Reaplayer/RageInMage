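; Player lightning gameplay ability for Ceaseless Wrath, a zone spell placed by aiming within max spell range.
; An aim-mode task drives a Niagara circle indicator, sized to the zone radius and tinted with the class color.
; On release it removes the indicator and commits, then faces the aim point and calls BeginCeaselessWrath there, or ends if the commit fails.
; Cancelling only removes the indicator.
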(event Ability|EventActivateAbility
  (bind _aimposition (|AimModeTask (Variables|Default|GetMaxSpellRange))
    (:OnAimUpdate
      (Utilities|IsValid (Variables|Default|GetIndicatorVFX)
        (:Is%20Valid
          _)
        (:Is%20Not%20Valid
          (bind _returnvalue (Niagara|SpawnSystematLocation "/Game/RageInMageSpells/VFX/Aim/NS_Aim_Circle.NS_Aim_Circle" (Transformation|GetActorLocation (Ability|GetAvatarActorfromActorInfo))))
          (bind _output_get (Variables|Default|SetIndicatorVFX _returnvalue))
          (Niagara|SetNiagaraVariable(Float) _output_get "Radius" (.Value (Utilities|Struct|BreakScalableFloat (Variables|Default|GetZoneRadius))))
          (bind _returnvalue_2 (Class|CombatInterface|GetCharacterClass(Message) (Ability|GetAvatarActorfromActorInfo)))
          (Niagara|SetNiagaraVariable(LinearColor) (Variables|Default|GetIndicatorVFX) "RingColour" (Class|RageinMageAbilitySystemLibrary|GetClassProgressBarColor _returnvalue_2))))
      (Transformation|SetWorldLocation (Variables|Default|GetIndicatorVFX) _aimposition false false))
    (:OnInputReleased
      (Utilities|IsValid (Variables|Default|GetIndicatorVFX)
        (:Is%20Valid
          (Components|Activation|Deactivate (Variables|Default|GetIndicatorVFX))
          (Components|DestroyComponent (Variables|Default|GetIndicatorVFX))
          (Variables|Default|SetIndicatorVFX 0)
          (bind _returnvalue_3 (Ability|CommitAbility))
          (if _returnvalue_3
            (Class|CombatInterface|UpdateFacingTarget(Message) (Ability|GetAvatarActorfromActorInfo) _aimposition)
            (Class|RageinMageCeaselessWrathAbility|BeginCeaselessWrath _aimposition)
            (else
              (Ability|EndAbility))))))
    (:OnCancelled
      (Utilities|IsValid (Variables|Default|GetIndicatorVFX)
        (:Is%20Valid
          (Components|Activation|Deactivate (Variables|Default|GetIndicatorVFX))
          (Components|DestroyComponent (Variables|Default|GetIndicatorVFX))
          (Variables|Default|SetIndicatorVFX 0))))))

(event Ability|EventOnEndAbility
  (params (bWasCancelled :type Boolean)))