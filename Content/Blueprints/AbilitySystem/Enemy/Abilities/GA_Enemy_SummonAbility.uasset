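; Enemy gameplay ability that summons minions around the avatar, capped by its maximum summon count.
; On activation it trims the summon amount to the remaining slots, gets and shuffles spawn locations, plays effects there and starts the avatar's summon montage.
; The montage event starts a loop that spawns and registers minions with short delays, rechecking the cap each time.
; Interrupting or cancelling the montage sets a flag checked by that loop.
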(event Ability|EventActivateAbility
  (bind _returnvalue (Ability|GetAvatarActorfromActorInfo))
  (bind _returnvalue_2 (Ability|GetAvatarActorfromActorInfo))
  (Variables|Default|SetCompleted false)
  (Variables|Default|SetToBeSummonedAmount (Variables|Default|GetSummonAmount))
  (bind _returnvalue_3 (Class|CombatInterface|GetSummonCount(Message) _returnvalue_2))
  (Variables|Default|SetSummonCount _returnvalue_3)
  (bind _returnvalue_4 (Class|CombatInterface|GetMaxSummonCount(Message) _returnvalue_2))
  (Variables|Default|SetMaxSummonCount _returnvalue_4)
  (if (<= (+ (Variables|Default|GetToBeSummonedAmount) (Variables|Default|GetSummonCount)) (Variables|Default|GetMaxSummonCount))
    _
    (else
      (Variables|Default|SetToBeSummonedAmount (- (Variables|Default|GetMaxSummonCount) (Variables|Default|GetSummonCount)))))
  (bind _returnvalue_5 (Class|RageinMageSummonGameplayAbility|GetSummonLocations (Variables|Default|GetToBeSummonedAmount)))
  (bind _output_get (Variables|Default|SetSpawnLocations _returnvalue_5))
  (Utilities|Array|Shuffle _output_get)
  (bind _returnvalue_6 (Class|CombatInterface|GetRandomAttackMontage(Message) (Ability|GetAvatarActorfromActorInfo) false true))
  (for _array_element _output_get
    (Niagara|SpawnSystematLocation (.SummonEffect (Utilities|Struct|BreakTaggedMontage _returnvalue_6)) _array_element))
  (|PlayMontageandWaitProxy "None" (.Montage (Utilities|Struct|BreakTaggedMontage _returnvalue_6)) 1.0 "None" true 1.0 0.0 false
    (:then
      (Ability|Tasks|WaitGameplayEvent (.MontageEventTag (Utilities|Struct|BreakTaggedMontage _returnvalue_6)) 0 true
        (:EventReceived
          (while (not (Variables|Default|GetCompleted))
            (bind _returnvalue_7 (Class|CombatInterface|GetSummonCount(Message) _returnvalue :!label _label))
            (bind _returnvalue_8 (Class|CombatInterface|GetMaxSummonCount(Message) _returnvalue))
            (if (< _returnvalue_7 _returnvalue_8)
              (if (< (Variables|Default|GetSpawnLocationIndex) (Utilities|Array|Length (Variables|Default|GetSpawnLocations)))
                (bind _returnvalue_9 (Game|SpawnActorfromClass (.SummonClass (Utilities|Struct|BreakTaggedMontage _returnvalue_6)) (Math|Transform|MakeTransform (+ (Utilities|Array|Get(acopy) (Variables|Default|GetSpawnLocations) (Variables|Default|GetSpawnLocationIndex)) "0.000000,0.000000,-40.000000") (Math|Rotator|FindLookatRotation (Transformation|GetActorLocation (Ability|GetAvatarActorfromActorInfo)) (+ (Utilities|Array|Get(acopy) (Variables|Default|GetSpawnLocations) (Variables|Default|GetSpawnLocationIndex)) "0.000000,0.000000,-40.000000")) "1.000000,1.000000,1.000000") "AlwaysSpawn" "MultiplyWithRoot" 0 0))
                (Class|CombatInterface|RegisterSpawnedMinion(Message) (Ability|GetAvatarActorfromActorInfo) _returnvalue_9)
                (Math|Integer|IncrementInt (Variables|Default|GetSpawnLocationIndex)
                  (:%20%20
                    (Utilities|FlowControl|Delay 0.2)
                    (goto _label)))
                (else
                  _)))
            (Variables|Default|SetCompleted true))
          (Ability|EndAbility))))
    (:OnInterrupted
      (Variables|Default|SetCompleted true :!label _label_2))
    (:OnCancelled
      (goto _label_2))))