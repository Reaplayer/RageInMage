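; Enemy melee attack gameplay ability that turns toward the combat target and plays a random attack montage.
; The montage's gameplay event triggers a debug-drawn radius check at the combat socket, damaging non-friendly live players and firing a melee impact cue on a hit.
; A motion-warping stop event adds a replicated loose tag, removed when the montage ends.
; An unconnected attack-sphere collision chain never runs.
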(event Ability|EventActivateAbility
  (bind _returnvalue (Ability|GetAvatarActorfromActorInfo))
  (bind _returnvalue_2 (Ability|GetAvatarActorfromActorInfo))
  (bind _returnvalue_3 (Ability|GetAvatarActorfromActorInfo))
  (Variables|Default|SetHasImpact false)
  (bind _returnvalue_4 (Class|CombatInterface|GetCombatSocketLocation(Message) _returnvalue_3 (.SocketTag (Utilities|Struct|BreakTaggedMontage (Variables|Default|GetTaggedMontage)))))
  (Variables|Default|SetCombatSocketLocation _returnvalue_4)
  (bind _returnvalue_5 (Class|EnemyInterface|GetCombatTarget(Message) _returnvalue_3))
  (Class|CombatInterface|UpdateFacingTarget(Message) _returnvalue_3 (Transformation|GetActorLocation _returnvalue_5))
  (bind _returnvalue_6 (Class|CombatInterface|GetAttackMontages(Message) _returnvalue_3))
  (bind _output_get (Variables|Default|SetTaggedMontage (Class|RageinMageDamageGameplayAbility|GetRandomTaggedMontagefromArray _returnvalue_6)))
  (|PlayMontageandWaitProxy "None" (.Montage (Utilities|Struct|BreakTaggedMontage _output_get)) 1.0 "None" false 1.0 0.0 false
    (:then
      (Ability|Tasks|WaitGameplayEvent (.MontageEventTag (Utilities|Struct|BreakTaggedMontage _output_get)) 0
        (:then
          (bind _payload (Ability|Tasks|WaitGameplayEvent "(TagName=\"Event.MotionWarping.Stop\")" 0)
            (:EventReceived
              (Ability|GameplayEffect|AddLooseGameplayTags _returnvalue (GameplayTags|MakeGameplayTagContainerfromTag (.EventTag (Utilities|Struct|BreakGameplayEventData _payload))) true))))
        (:EventReceived
          (bind _returnvalue_7 (Class|CombatInterface|GetCombatSocketLocation(Message) (Ability|GetAvatarActorfromActorInfo) (.SocketTag (Utilities|Struct|BreakTaggedMontage _output_get))))
          (bind _output_get_2 (Variables|Default|SetCombatSocketLocation _returnvalue_7))
          (Rendering|Debug|DrawDebugSphere _output_get_2 35.0 12 "(R=0.013069,G=1.000000,B=0.052179,A=1.000000)" 1.0)
          (bind _outoverlappingactors (Class|RageinMageAbilitySystemLibrary|GetLivePlayersWithinRadius _returnvalue_2 35.0 (Utilities|Array|MakeArray _returnvalue_2) _output_get_2))
          (for _array_element _outoverlappingactors
            (bind _returnvalue_8 (Class|RageinMageAbilitySystemLibrary|IsFriendly (Ability|GetAvatarActorfromActorInfo) _array_element))
            (if (not _returnvalue_8)
              (Class|RageinMageDamageGameplayAbility|CauseDamage _array_element)
              (Variables|Default|SetHasImpact true)))
          (if (Variables|Default|GetHasImpact)
            (bind _returnvalue_9 (Class|EnemyInterface|GetCombatTarget(Message) (Ability|GetAvatarActorfromActorInfo)))
            (Class|GameplayAbility|ExecuteGameplayCuewithParams "(TagName=\"GameplayCue.MeleeImpact\")" (Ability|GameplayCue|MakeGameplayCueParameters :Location (Variables|Default|GetCombatSocketLocation) :SourceObject _returnvalue_9))))))
    (:OnCompleted
      (Ability|EndAbility :!label _label)
      (Ability|GameplayEffect|RemoveLooseGameplayTags _returnvalue (GameplayTags|MakeGameplayTagContainerfromTag (.EventTag (Utilities|Struct|BreakGameplayEventData _payload))) true))
    (:OnInterrupted
      (goto _label))
    (:OnCancelled
      (goto _label))))