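; Enemy ranged attack ability that turns the avatar toward its combat target and fires a projectile at it during an attack montage.
; It plays a random tagged montage and spawns the projectile when that montage's gameplay event arrives, aimed at the target's location.
; A motion-warping stop event adds its tag to the avatar as a replicated loose tag, removed when the montage completes, is interrupted or is cancelled, as the ability ends.
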(event Ability|EventActivateAbility
  (bind _returnvalue (Ability|GetAvatarActorfromActorInfo))
  (bind _returnvalue_2 (Ability|GetAvatarActorfromActorInfo))
  (bind _returnvalue_3 (Class|EnemyInterface|GetCombatTarget(Message) _returnvalue_2))
  (Class|CombatInterface|UpdateFacingTarget(Message) _returnvalue_2 (Transformation|GetActorLocation _returnvalue_3))
  (bind _returnvalue_4 (Class|CombatInterface|GetAttackMontages(Message) _returnvalue_2))
  (bind _output_get (Variables|Default|SetTaggedMontage (Class|RageinMageDamageGameplayAbility|GetRandomTaggedMontagefromArray _returnvalue_4)))
  (|PlayMontageandWaitProxy "None" (.Montage (Utilities|Struct|BreakTaggedMontages _output_get)) 1.0 "None" false 1.0 0.0 false
    (:then
      (Ability|Tasks|WaitGameplayEvent (.MontageTag (Utilities|Struct|BreakTaggedMontages _output_get)) 0
        (:then
          (bind _payload (Ability|Tasks|WaitGameplayEvent "(TagName=\"Event.MotionWarping.Stop\")" 0)
            (:EventReceived
              (Ability|GameplayEffect|AddLooseGameplayTags _returnvalue (GameplayTags|MakeGameplayTagContainerfromTag (.EventTag (Utilities|Struct|BreakGameplayEventData _payload))) true))))
        (:EventReceived
          (Class|RageinMageProjectileSpell|SpawnProjectile (Transformation|GetActorLocation _returnvalue_3)))))
    (:OnCompleted
      (Ability|EndAbility :!label _label)
      (Ability|GameplayEffect|RemoveLooseGameplayTags _returnvalue (GameplayTags|MakeGameplayTagContainerfromTag (.EventTag (Utilities|Struct|BreakGameplayEventData _payload))) true))
    (:OnInterrupted
      (goto _label))
    (:OnCancelled
      (goto _label))))

(event Ability|EventOnEndAbility
  (params (bWasCancelled :type Boolean)))