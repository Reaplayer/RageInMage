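; Enemy ranged attack gameplay ability that fires a projectile at the avatar's combat target.
; It starts tracking and facing the target, picks a random ranged montage, then plays it after a short delay.
; The montage's tagged event spawns its projectile from the tagged socket with calculated pitch and target leading.
; A motion-warping stop event adds a replicated loose tag, removed when the montage completes or aborts and the ability ends.
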(event Ability|EventActivateAbility
  (bind _returnvalue (Ability|GetAvatarActorfromActorInfo))
  (bind _returnvalue_2 (Ability|GetAvatarActorfromActorInfo))
  (bind _returnvalue_3 (Class|EnemyInterface|GetCombatTarget(Message) _returnvalue_2))
  (bind _output_get (Variables|Default|SetCombatTarget _returnvalue_3))
  (Class|RageinMageProjectileSpell|StartTrackingTarget _output_get)
  (Class|CombatInterface|UpdateFacingTarget(Message) _returnvalue_2 (Transformation|GetActorLocation _returnvalue_3))
  (bind _returnvalue_4 (Class|CombatInterface|GetRandomAttackMontage(Message) _returnvalue_2 true false))
  (bind _output_get_2 (Variables|Default|SetTaggedMontage _returnvalue_4))
  (Ability|Tasks|WaitDelay 1.0
    (:OnFinish
      (|PlayMontageandWaitProxy "None" (.Montage (Utilities|Struct|BreakTaggedMontage _output_get_2)) 1.0 "None" false 1.0 0.0 false
        (:then
          (Ability|Tasks|WaitGameplayEvent (.MontageEventTag (Utilities|Struct|BreakTaggedMontage _output_get_2)) 0 true
            (:then
              (bind _payload (Ability|Tasks|WaitGameplayEvent "(TagName=\"Event.MotionWarping.Stop\")" 0 true)
                (:EventReceived
                  (bind _output_get_3 (Variables|Default|SetMotionWarpingStopTag (GameplayTags|MakeGameplayTagContainerfromTag (.EventTag (Utilities|Struct|BreakGameplayEventData _payload)))))
                  (Ability|GameplayEffect|AddLooseGameplayTags _returnvalue _output_get_3 true))))
            (:EventReceived
              (Class|RageinMageProjectileSpell|SpawnProjectile (Transformation|GetActorLocation _returnvalue_3) (.SocketTag (Utilities|Struct|BreakTaggedMontage _output_get_2)) (.ProjectileClass (Utilities|Struct|BreakTaggedMontage _output_get_2)) true (Variables|Default|GetCombatTarget)))))
        (:OnCompleted
          (Ability|GameplayEffect|RemoveLooseGameplayTags _returnvalue (Variables|Default|GetMotionWarpingStopTag) true :!label _label)
          (Ability|EndAbility))
        (:OnInterrupted
          (goto _label))
        (:OnCancelled
          (goto _label))))))