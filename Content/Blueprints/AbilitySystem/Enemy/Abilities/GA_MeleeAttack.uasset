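; Enemy melee attack ability that warps to face the combat target and plays a random tagged attack montage.
; The montage's gameplay event triggers a small sphere query at the tag's combat socket, drawn for debug, damaging live players inside.
; A parallel wait turns the motion-warping stop event into a replicated loose tag on the avatar.
; Montage completion, interruption or cancellation ends the ability and removes that tag.
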(event Ability|EventActivateAbility
  (bind _returnvalue (Ability|GetAvatarActorfromActorInfo))
  (bind _returnvalue_2 (Ability|GetAvatarActorfromActorInfo))
  (bind _returnvalue_3 (Ability|GetAvatarActorfromActorInfo))
  (bind _returnvalue_4 (Class|EnemyInterface|GetCombatTarget(Message) _returnvalue))
  (Class|CombatInterface|UpdateFacingTarget(Message) _returnvalue (Transformation|GetActorLocation _returnvalue_4))
  (bind _returnvalue_5 (Class|CombatInterface|GetAttackMontages(Message) _returnvalue))
  (bind _output_get (Variables|Default|SetTaggedMontage (Class|RageinMageDamageGameplayAbility|GetRandomTaggedMontagefromArray _returnvalue_5)))
  (|PlayMontageandWaitProxy "None" (.Montage (Utilities|Struct|BreakTaggedMontages _output_get)) 1.0 "None" false 1.0 0.0 false
    (:then
      (Ability|Tasks|WaitGameplayEvent (.MontageTag (Utilities|Struct|BreakTaggedMontages _output_get)) 0
        (:then
          (bind _payload (Ability|Tasks|WaitGameplayEvent "(TagName=\"Event.MotionWarping.Stop\")" 0)
            (:EventReceived
              (Ability|GameplayEffect|AddLooseGameplayTags _returnvalue_2 (GameplayTags|MakeGameplayTagContainerfromTag (.EventTag (Utilities|Struct|BreakGameplayEventData _payload))) true))))
        (:EventReceived
          (bind _returnvalue_6 (Class|CombatInterface|GetCombatSocketLocation(Message) (Ability|GetAvatarActorfromActorInfo) (.MontageTag (Utilities|Struct|BreakTaggedMontages _output_get))))
          (Rendering|Debug|DrawDebugSphere _returnvalue_6 35.0 12 "(R=0.013069,G=1.000000,B=0.052179,A=1.000000)" 1.0)
          (bind _outoverlappingactors (Class|RageinMageAbilitySystemLibrary|GetLivePlayersWithinRadius _returnvalue_3 35.0 (Utilities|Array|MakeArray _returnvalue_3) _returnvalue_6))
          (for _array_element _outoverlappingactors
            (Class|RageinMageDamageGameplayAbility|CauseDamage _array_element)))))
    (:OnCompleted
      (Ability|EndAbility :!label _label)
      (Ability|GameplayEffect|RemoveLooseGameplayTags _returnvalue_2 (GameplayTags|MakeGameplayTagContainerfromTag (.EventTag (Utilities|Struct|BreakGameplayEventData _payload))) true))
    (:OnInterrupted
      (goto _label))
    (:OnCancelled
      (goto _label))))