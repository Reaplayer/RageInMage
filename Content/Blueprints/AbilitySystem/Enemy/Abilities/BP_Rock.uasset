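; BP_Rock is a rock actor for enemy abilities that tumbles visually while active.
; On BeginPlay it picks random pitch, roll and yaw rates, which Tick applies to RockMesh as a frame-rate-independent local rotation.
; BeginPlay also waits briefly before setting the Sphere's collision to query-only.
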(event EventBeginPlay
  (bind _returnvalue (Math|Random|RandomFloatinRange -5e+02 5e+02))
  (Variables|Default|SetPitchRotationRate _returnvalue)
  (Variables|Default|SetRollRotationRate _returnvalue)
  (Variables|Default|SetYaw%20RotationRate _returnvalue)
  (Utilities|FlowControl|Delay 0.1)
  (Collision|SetCollisionEnabled (Variables|Default|GetSphere) "QueryOnly"))

(event EventTick
  (params (DeltaSeconds :type Float%20%28single-precision%29))
  (Transformation|AddLocalRotation (Variables|Default|GetRockMesh) (Math|Rotator|MakeRotator (* DeltaSeconds (Variables|Default|GetRollRotationRate)) (* DeltaSeconds (Variables|Default|GetPitchRotationRate)) (* DeltaSeconds (Variables|Default|GetYaw%20RotationRate))) false false))

(fn ConstructionScript)