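; Enemy melee attack ability that plays a random montage facing the combat target and supports repeated hit checks during the swing.
; Each montage event sphere-checks the combat socket for live players, damages non-friendly ones and fires a melee impact cue.
; ActorsAlreadyHit is meant to prevent repeat hits, though its nested-loop comparison only guarantees this with one recorded actor.
; A motion-warping stop event adds a loose tag, removed when the montage ends.
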(event Ability|EventActivateAbility
  (bind _returnvalue (Ability|GetAvatarActorfromActorInfo))
  (bind _returnvalue_2 (Ability|GetAvatarActorfromActorInfo))
  (bind _returnvalue_3 (Ability|GetAvatarActorfromActorInfo))
  (bind _returnvalue_4 (Ability|GetAvatarActorfromActorInfo))
  (Utilities|Array|Clear (Variables|Default|GetActorsAlreadyHit))
  (Variables|Default|SetHasImpact false)
  (bind _returnvalue_5 (Class|EnemyInterface|GetCombatTarget(Message) _returnvalue))
  (Class|CombatInterface|UpdateFacingTarget(Message) _returnvalue (Transformation|GetActorLocation _returnvalue_5))
  (bind _returnvalue_6 (Class|CombatInterface|GetRandomAttackMontage(Message) _returnvalue false false))
  (bind _output_get (Variables|Default|SetTaggedMontage _returnvalue_6))
  (|PlayMontageandWaitProxy "None" (.Montage (Utilities|Struct|BreakTaggedMontage _output_get)) 1.0 "None" false 1.0 0.0 false
    (:then
      (Ability|Tasks|WaitGameplayEvent (.MontageEventTag (Utilities|Struct|BreakTaggedMontage _output_get)) 0
        (:then
          (bind _payload (Ability|Tasks|WaitGameplayEvent "(TagName=\"Event.MotionWarping.Stop\")" 0)
            (:EventReceived
              (bind _output_get_2 (Variables|Default|SetMotionWarpingStopTag (GameplayTags|MakeGameplayTagContainerfromTag (.EventTag (Utilities|Struct|BreakGameplayEventData _payload)))))
              (Ability|GameplayEffect|AddLooseGameplayTags _returnvalue_2 _output_get_2 true))))
        (:EventReceived
          (bind _returnvalue_7 (Class|CombatInterface|GetCombatSocketLocation(Message) (Ability|GetAvatarActorfromActorInfo) (.SocketTag (Utilities|Struct|BreakTaggedMontage _output_get))))
          (bind _output_get_3 (Variables|Default|SetCombatSocketLocation _returnvalue_7))
          (bind _outoverlappingactors (Class|RageinMageAbilitySystemLibrary|GetLivePlayersWithinRadius _returnvalue_3 35.0 (Utilities|Array|MakeArray _returnvalue_3) _output_get_3))
          (for _array_element _outoverlappingactors
            (if (> (Utilities|Array|Length (Variables|Default|GetActorsAlreadyHit)) 0)
              (for _array_element_2 (Variables|Default|GetActorsAlreadyHit)
                (if (not (== _array_element_2 _array_element))
                  (bind _returnvalue_8 (Class|RageinMageAbilitySystemLibrary|IsFriendly (Ability|GetAvatarActorfromActorInfo) _array_element))
                  (if (not _returnvalue_8)
                    (Class|RageinMageDamageGameplayAbility|CauseDamage _array_element)
                    (Variables|Default|SetHasImpact true)
                    (Utilities|Array|Add (Variables|Default|GetActorsAlreadyHit) _array_element))))
              (else
                (bind _returnvalue_9 (Class|RageinMageAbilitySystemLibrary|IsFriendly (Ability|GetAvatarActorfromActorInfo) _array_element))
                (if (not _returnvalue_9)
                  (Class|RageinMageDamageGameplayAbility|CauseDamage _array_element)
                  (Variables|Default|SetHasImpact true)
                  (Utilities|Array|Add (Variables|Default|GetActorsAlreadyHit) _array_element)))))
          (if (Variables|Default|GetHasImpact)
            (bind _returnvalue_10 (Class|EnemyInterface|GetCombatTarget(Message) _returnvalue_4))
            (Class|GameplayAbility|ExecuteGameplayCuewithParams "(TagName=\"GameplayCue.MeleeImpact\")" (Ability|GameplayCue|MakeGameplayCueParameters :AggregatedSourceTags (GameplayTags|MakeGameplayTagContainerfromTag (.MontageEventTag (Utilities|Struct|BreakTaggedMontage (Variables|Default|GetTaggedMontage)))) :Location (Variables|Default|GetCombatSocketLocation) :EffectCauser _returnvalue_4 :SourceObject _returnvalue_10))
            (Variables|Default|SetHasImpact false)))))
    (:OnCompleted
      (Ability|EndAbility :!label _label)
      (Ability|GameplayEffect|RemoveLooseGameplayTags _returnvalue_2 (Variables|Default|GetMotionWarpingStopTag) true))
    (:OnInterrupted
      (goto _label))
    (:OnCancelled
      (goto _label))))